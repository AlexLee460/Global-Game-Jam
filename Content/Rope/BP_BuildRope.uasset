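; BP_BuildRope is an actor that starts building a physics rope from a start actor toward a hit point.
; On BeginPlay it takes a start point raised above that actor and the hit's impact point as the end.
; It spawns the first BP_RopeSegment facing the end and joins its mesh to the start actor's physics constraint.
; It derives a segment count from hit distance and mesh length, but spawns no further segments.
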(event `self.ReceiveBeginPlay`
  (bind (_bblockinghit _binitialoverlap _time _distance _location _impactpoint _normal _impactnormal _physmat _hitactor) (`GameplayStatics.BreakHitResult` (`self.Hit Result`)))
  (bind _start_actor_to_attach (`self.Start Actor to Attach`)
    (:`then`
      (`KismetSystemLibrary.PrintString` "Actor Valid")
      (bind (_returnvalue_x _returnvalue_y _returnvalue_z) (`KismetMathLibrary.BreakVector` (`self.K2_GetActorLocation` _start_actor_to_attach)))
      (set `self.StartPoint` (`KismetMathLibrary.MakeVector` _returnvalue_x _returnvalue_y (+ _returnvalue_z 65.0)))
      (`/Engine/EditorBlueprintResources/StandardMacros.IsValid` _hitactor
        (:`Is Valid`
          (`KismetSystemLibrary.PrintString` "Actor Valid")
          (set `self.EndPoint` _impactpoint)
          (`self.StartBuildingRope` (`self.Hit Result`) (`self.Start Actor to Attach`)))))
    (:`else`)))

(fn `SetNumberOfSegments`
  (params (Distance :type "Float (double-precision)"))
  (set `self.Number of segments` (`KismetMathLibrary.Round` (/ Distance (`self.RopeMeshLength`)))))

(fn `StartBuildingRope`
  (params (`Hit Result` :type "HitResult Structure") (StartActorToAttach :type "Actor Object Reference"))
  (bind (_bblockinghit _binitialoverlap _time _distance _location _impactpoint _normal _impactnormal _physmat _hitactor) (`GameplayStatics.BreakHitResult` `Hit Result`))
  (`/Engine/EditorBlueprintResources/StandardMacros.IsValid` _hitactor
    (:`Is Valid`
      (`|ExecutionSequence`
        (:`then_0`
          (`self.SpawnFirstSegment` StartActorToAttach))
        (:`then_1`
          (`self.SetNumberOfSegments` _distance))))))

(fn `UserConstructionScript`)